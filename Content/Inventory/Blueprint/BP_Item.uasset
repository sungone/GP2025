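; BP_Item is an item actor that shows the mesh for its item ID.
; Its construction script looks up the item's row name in GPItemTable and uses the static mesh if valid, hiding the skeletal mesh component.
; Otherwise it assigns the row's skeletal mesh, shows it and hides the static mesh component.
; The event graph holds only empty default events, so the Blueprint adds no runtime logic.
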(event EventBeginPlay)

(event Collision|EventActorBeginOverlap
  (params (OtherActor :type Actor%20Object%20Reference)))

(event EventTick
  (params (DeltaSeconds :type Float%20%28single-precision%29)))

(fn ConstructionScript
  (bind _returnvalue (Utilities|GetDataTableRow "/Game/Item/GPItemTable.GPItemTable" (.rowname (.itemid (Variables|Item|GetItem))))
    (:then
      (Utilities|IsValid (.itemstaticmesh _returnvalue)
        (:Is%20Valid
          (Components|StaticMesh|SetStaticMesh (Variables|Default|GetItemStaticMesh) (.itemstaticmesh _returnvalue))
          (Rendering|SetVisibility (Variables|Default|GetItemSkeletalMesh) false false))
        (:Is%20Not%20Valid
          (Components|SkeletalMesh|SetSkeletalMeshAsset (Variables|Default|GetItemSkeletalMesh) (.itemskeletalmesh _returnvalue))
          (Rendering|SetVisibility (Variables|Default|GetItemSkeletalMesh) true false)
          (Rendering|SetVisibility (Variables|Default|GetItemStaticMesh) false false))))))