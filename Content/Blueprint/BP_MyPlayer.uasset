(event EventBeginPlay
  ;[1 1 1] NavMesh 추출
  (bind _asgpgame_instance (Utilities|Casting|CastToGPGameInstance (Game|GetGameInstance)))
  (Class|GPGameInstance|SaveNavData _asgpgame_instance false)
  ;[1 1 1] 인벤토리 플레이어 캡처
  (CallFunction|UpdateSceneCaptureComponents)
  (Rendering|SceneCapture|CaptureScene (Variables|Default|GetPlayerCapture) :!class /Script/Engine.SceneCaptureComponent2D)
  ;[1 1 1] 지도 캡처
  (bind _outactors (Actor|GetAllActorsOfClass "/Game/UI/Texture/Map/BP_MapCapture.BP_MapCapture_C"))
  (for _array_element _outactors
    (if (Actor|ActorHasTag _array_element "MapCapture")
      (Variables|SceneCapture|SetBPMapCaptureRef _array_element)
      (else
        (Development|PrintString "MapCaptureRefFailed"))))
  (Development|PrintString "MapCaptureRefFailed"))

(event Collision|EventActorBeginOverlap
  (params (OtherActor :type Actor%20Object%20Reference)))

(event EventTick
  (params (DeltaSeconds :type Float%20%28single-precision%29)))

(event Input|KeyboardEvents|M
  (params (Key :type Key%20Structure :default "None"))
  (:Pressed
    (Rendering|SceneCapture|CaptureScene (Variables|/Game/UI/Texture/Map/BP_MapCapture.BP_MapCapture_C|GetSceneCaptureComponent2D (Variables|SceneCapture|GetBPMapCaptureRef)) :!class /Script/Engine.SceneCaptureComponent2D)
    (bind _returnvalue (UserInterface|CreateWidget "/Game/UI/WBP_Map.WBP_Map_C" (Game|GetPlayerController 0)))
    (UserInterface|Viewport|AddtoViewport _returnvalue 0))
  (:Released
    (Widget|RemovefromParent _returnvalue)))

(event Input|KeyboardEvents|I
  (params (Key :type Key%20Structure :default "None"))
  ;[1 1 1] e동 체육관 순간이동
  (:Pressed
    (Transformation|SetActorLocation self "-4798.570000,-12678.820000,942.810000" false false)
    (Development|PrintString "Teleport to E")))

(event Input|KeyboardEvents|O
  (params (Key :type Key%20Structure :default "None"))
  ;[1 1 1] e동 체육관 순간이동
  (:Pressed
    (Transformation|SetActorLocation self "-4009.940000,5271.430000,146.280000" false false)
    (Development|PrintString "Teleport to GYM")))

(fn ConstructionScript)

(fn UpdateSceneCaptureComponents
  (bind _playercapture (Variables|Default|GetPlayerCapture))
  (Rendering|SceneCapture|ClearShowOnlyComponents _playercapture)
  (Rendering|SceneCapture|ShowOnlyComponent _playercapture (Variables|Default|GetBodyMesh))
  (Rendering|SceneCapture|ShowOnlyComponent _playercapture (Variables|Default|GetHelmet))
  (Rendering|SceneCapture|ShowOnlyComponent _playercapture (Variables|Default|GetHeadMesh))
  (Rendering|SceneCapture|ShowOnlyComponent _playercapture (Variables|Default|GetLegMesh)))